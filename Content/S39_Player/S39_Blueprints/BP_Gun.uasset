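; BP_Gun is a Colt 45 pickup for S39_MainChar that sets default ammo, capacity and damage on BeginPlay.
; Unless disabled, PickupColt45 grants the gun to a character without one, copies Ammo over and calls Interacted.
; If the character already owns it, a random count up to a full magazine overwrites their ammo instead of adding to it, and Interacted is skipped.
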(event `self.ReceiveBeginPlay`
  (set `self.Ammo` 8)
  (set `self.Capacity` 8)
  (set `self.Damage` 10))

(event `Pickup Colt45`
  (params (Interactor :type "Actor Object Reference"))
  (if (not (`self.Disable`))
    (bind _ass39_main_char (cast `/Game/S39_Player/S39_MainChar` Interactor))
    (if (`/Game/S39_Player/S39_MainChar.Colt45` _ass39_main_char)
      (bind _output_get (set `self.Ammo` (`KismetMathLibrary.RandomIntegerInRange` 0 8)))
      (set `/Game/S39_Player/S39_MainChar.Ammo_Colt45` _output_get _ass39_main_char)
      (else
        (set `/Game/S39_Player/S39_MainChar.Colt45` true _ass39_main_char)
        (set `/Game/S39_Player/S39_MainChar.Ammo_Colt45` (`self.Ammo`) _ass39_main_char)
        (`self.Interacted`)))))

(fn `UserConstructionScript`
  (`parent.UserConstructionScript`))